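; PlayerOrbBP is an orb actor that follows the player and grows as orbs are counted.
; Each tick it copies the transform of the player character's static mesh component tagged "Orb".
; Its sphere bobs vertically by accumulating a speed offset that reverses beyond a fixed range.
; NewOrb increments the orb counter, plays an eject sound and scales the sphere in proportion to the count.
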(event `self.ReceiveBeginPlay`)

(event `self.ReceiveTick`
  (params (DeltaSeconds :type "Float (single-precision)"))
  (bind _speed (`self.Speed`))
  (`self.K2_SetActorTransform` (`SceneComponent.K2_GetComponentToWorld` (`|GetArrayItem` (`self.GetComponentsByTag` (`GameplayStatics.GetPlayerCharacter` 0) "/Script/Engine.StaticMeshComponent" "Orb"))))
  (bind _output_get (set `self.Movement` (+ _speed (`self.Movement`))))
  (`SceneComponent.K2_AddWorldOffset` (`self.Sphere`) (`KismetMathLibrary.MakeVector` 0.0 0.0 _speed) false false)
  (if (> (`KismetMathLibrary.Abs` _output_get) 1.5)
    (set `self.Speed` (* (`self.Speed`) -1.0))))

(fn `NewOrb`
  (bind _output_get (set `self.OrbCounter` (+ (`self.OrbCounter`) 1)))
  (`GameplayStatics.PlaySound2D` "/Engine/EditorSounds/GamePreview/EjectFromPlayer.EjectFromPlayer" 1.0 1.0 0.0 null null)
  (`SceneComponent.SetWorldScale3D` (`self.Sphere`) (* _output_get (0.05 0.05 0.05))))

(fn `UserConstructionScript`)