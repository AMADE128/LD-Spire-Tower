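; PortalBP is a portal actor that moves the player character to another portal sharing its PortalIndex.
; When the player overlaps the Portal component, it searches all PortalBP actors for matching indices other than itself.
; It sets the player's location to the match's ExitReference, keeping the world-space offset from the entered portal and leaving rotation untouched.
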(event `self.Portal.OnComponentBeginOverlap`
  (params (OverlappedComponent :type "PrimitiveComponent Object Reference") (OtherActor :type "Actor Object Reference") (OtherComp :type "PrimitiveComponent Object Reference") (OtherBodyIndex :type Integer) (bFromSweep :type Boolean) (SweepResult :type "HitResult Structure (by ref)"))
  (if (== OtherActor (`GameplayStatics.GetPlayerCharacter` 0))
    (if true
      (bind _outactors (`GameplayStatics.GetAllActorsOfClass` "PortalBP_C"))
      (for _array_element _outactors
        (if (== (`/Game/PortalBP.PortalIndex` _array_element) (`self.PortalIndex`))
          (if (!= _array_element self)
            (`self.K2_SetActorLocation` OtherActor (- (`SceneComponent.K2_GetComponentLocation` (`/Game/PortalBP.ExitReference` _array_element)) (- (`SceneComponent.K2_GetComponentLocation` (`self.Portal`)) (`self.K2_GetActorLocation` OtherActor))) false false)))))))

(fn `UserConstructionScript`)